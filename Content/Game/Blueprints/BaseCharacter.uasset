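; Base multiplayer player character with movement, aiming, jumping and a Pistol, Rifle and Shotgun inventory.
; Local ticks send aim yaw to the server, and aim state replicates through server calls.
; Weapon switching multicasts an equip montage, then the server selects the slot and applies DataTable stats, mesh and animation assets.
; Shooting is a local debug line trace with effects; its montage path is unused, and reload uses hard-coded pistol montages.
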(event Custom|ServerAim
  (params (Aim :type Boolean))
  ;[0 0.3343 0.9271] Replicated aiming
  (Variables|WeaponSetup|SetAim Aim))

(event Custom|DisableAllInput
  (params (PlayerController :type Player%20Controller%20Object%20Reference))
  ;[0 0.3343 0.9271] Not sure why this is needed
  (Input|DisableInput PlayerController))

(event Custom|MulticastSelectWeapon
  (params (WeaponName :type Name))
  ;[0 0.3343 0.9271] Replicated select weapon
  (CallFunction|WeaponEffects WeaponName))

(event Custom|SwitchWeapon
  (params (WeaponSlot :type Integer))
  ;[0 0.3343 0.9271] Replicated weapon switching
  (Networking|SwitchHasAuthority
    (:Authority
      (CallFunction|MulticastSwitchWeapon WeaponSlot))
    (:Remote
      (CallFunction|ServerSwitchWeapon WeaponSlot))))

(event Custom|ServerSwitchWeapon
  (params (WeaponSlot :type Integer))
  ;[0 0.3343 0.9271] Replicated weapon switching
  (CallFunction|MulticastSwitchWeapon WeaponSlot))

(event Custom|MulticastSwitchWeapon
  (params (WeaponSlot :type Integer))
  ;[0 0.3343 0.9271] Replicated weapon switching
  (if (== (Utilities|Array|Get(acopy) (Variables|WeaponSetup|GetWeaponInventory) WeaponSlot) "Pistol")
    (Variables|AnimationSetup|SetCharacterEquipAnim "/Game/Game/Assets/Animations/Retarget/AM_MM_Pistol_Equip.AM_MM_Pistol_Equip")
    (else
      (Variables|AnimationSetup|SetCharacterEquipAnim "/Game/Game/Assets/Animations/Retarget/AM_MM_Rifle_Equip.AM_MM_Rifle_Equip")))
  (Animation|Montage|PlayMontage (Variables|Character|GetMesh) (Variables|AnimationSetup|GetCharacterEquipAnim)
    (:then
      (if (Networking|IsServer)
        (Utilities|FlowControl|Delay 0.3)
        (CallFunction|ServerSelectWeapon WeaponSlot)))
    (:OnCompleted
      (Variables|WeaponSetup|SetSwitchingWeapon false))))

(event Custom|ServerSetYawOffet
  (params (NormalYawOffset :type Float%20%28single-precision%29))
  ;[0 0.3343 0.9271] Replicated rotation
  (Variables|CharacterSetup|SetNormalYawOffset NormalYawOffset))

(event Custom|PlayShootingMontage
  ;[0 0.3343 0.9271] Replicated shooting
  ;;[0.005208 0.005208 0.005208 0.542] Shooting montage looks wierd
  (Networking|SwitchHasAuthority
    (:Authority
      (CallFunction|MulticastShootingMontage))
    (:Remote
      (CallFunction|ServerShootingMontage))))

(event Custom|ServerShootingMontage
  ;[0 0.3343 0.9271] Replicated shooting
  (CallFunction|MulticastShootingMontage))

(event Custom|MulticastShootingMontage
  ;[0 0.3343 0.9271] Replicated shooting
  (Animation|Montage|PlayMontage (Variables|Character|GetMesh) "/Game/Game/Assets/Animations/Retarget/AM_MM_Pistol_Fire.AM_MM_Pistol_Fire"
    (:then
      (Animation|Montage|PlayMontage (Variables|Default|GetWeaponMesh) "/Game/Game/Weapons/Pistol/Animations/AM_Weap_Pistol_Fire.AM_Weap_Pistol_Fire"))))

(event Custom|PlayReloadMontage
  ;[0 0.3343 0.9271] Replicated reloading
  (Networking|SwitchHasAuthority
    (:Authority
      (CallFunction|MulticastReloadMontage))
    (:Remote
      (CallFunction|ServerReloadMonage))))

(event Custom|ServerReloadMonage
  ;[0 0.3343 0.9271] Replicated reloading
  (CallFunction|MulticastReloadMontage))

(event Custom|MulticastReloadMontage
  ;[0 0.3343 0.9271] Replicated reloading
  (Animation|Montage|PlayMontage (Variables|Character|GetMesh) "/Game/Game/Assets/Animations/Retarget/AM_MM_Pistol_Reload.AM_MM_Pistol_Reload"
    (:then
      (Animation|Montage|PlayMontage (Variables|Default|GetWeaponMesh) "/Game/Game/Weapons/Pistol/Animations/AM_Weap_Pistol_Reload.AM_Weap_Pistol_Reload"))
    (:OnCompleted
      (Variables|WeaponSetup|SetReload false))))

(event Custom|ServerSelectWeapon
  (params (WeaponSlot :type Integer))
  ;[0 0.3343 0.9271] Replicated select weapon
  (CallFunction|ServerReplicatedWeaponVariables WeaponSlot)
  (CallFunction|MulticastSelectWeapon (Utilities|Array|Get(acopy) (Variables|WeaponSetup|GetWeaponInventory) WeaponSlot)))

(event EventBeginPlay
  ;[0 0.3343 0.9271] Begin play
  (if (Pawn|IsLocallyControlled)
    (bind _asmain_player_controller (Utilities|Casting|CastToMainPlayerController (Game|GetPlayerController 0)))
    (Variables|Frameworksetup|SetMainGameWidget (Variables|/Game/Game/Blueprints/ModesAndControllers/MainPlayerController.MainPlayerController_C|GetMainGameWidget _asmain_player_controller))
    ;;[0.005208 0.005208 0.005208 0.542] Replicate weapon functions
    (CallFunction|ServerAddWeaponstoInventory 0 "Pistol")
    (CallFunction|ServerAddWeaponstoInventory 1 "Rifle")
    (CallFunction|ServerAddWeaponstoInventory 2 "Shotgun")
    (CallFunction|ServerSelectWeapon)
    (else
      (Actor|Tick|SetActorTickEnabled false))))

(event Collision|EventActorBeginOverlap
  (params (OtherActor :type Actor%20Object%20Reference)))

(event EventTick
  (params (DeltaSeconds :type Float%20%28single-precision%29))
  ;[0 0.3343 0.9271] Replicated rotation
  (if (Pawn|IsLocallyControlled)
    (Variables|Charactersetup|SetNewYawOffset (.yaw (Math|Rotator|Delta(Rotator) (Pawn|GetBaseAimRotation) (Transformation|GetActorRotation))))
    (Networking|SwitchHasAuthority
      (:Authority
        (Variables|Charactersetup|SetNewYawOffset (Variables|CharacterSetup|GetNormalYawOffset)))
      (:Remote
        (CallFunction|ServerSetYawOffet (Variables|Charactersetup|GetNewYawOffset))
        (Variables|CharacterSetup|SetNormalYawOffset (Variables|Charactersetup|GetNewYawOffset))))))

(event EventPossessed
  (params (NewController :type Controller%20Object%20Reference))
  ;[0 0.3343 0.9271] Not sure why this is needed
  (CallFunction|DisableAllInput (.AsMain%20Player%20Controller (Utilities|Casting|CastToMainPlayerController NewController))))

(event Input|ActionEvents|InputActionJump
  (params (Key :type Key%20Structure :default "None"))
  ;[0 0.3343 0.9271] Movement
  (:Pressed
    (Character|Jump))
  (:Released
    (Character|StopJumping)))

(event Input|ActionEvents|InputActionAim
  (params (Key :type Key%20Structure :default "None"))
  ;[0 0.3343 0.9271] Replicated aiming
  (:Pressed
    (Networking|SwitchHasAuthority
      (:Authority
        _)
      (:Remote
        (CallFunction|ServerAim true)))
    (Variables|WeaponSetup|SetAim true))
  (:Released
    (Networking|SwitchHasAuthority
      (:Authority
        _)
      (:Remote
        (CallFunction|ServerAim false)))
    (Variables|WeaponSetup|SetAim false)))

(event Input|ActionEvents|InputActionShoot
  (params (Key :type Key%20Structure :default "None"))
  (bind _weaponmesh (Variables|Default|GetWeaponMesh))
  (bind _returnvalue (Transformation|GetSocketTransform _weaponmesh "Muzzle" "RTS_World"))
  ;[0 0.3343 0.9271] Shooting
  (:Pressed
    (Effects|SpawnEmitterAttached 0 (Variables|Default|GetWeaponMesh) "Muzzle")
    (Audio|SpawnSound2D "/Game/Game/Assets/Audio/Sounds/Weapons/Rifle/Weapons_Rifle_Noise-Exterior-Distant_01.Weapons_Rifle_Noise-Exterior-Distant_01" 1.0 1.0 0.0 0)
    (Collision|LineTraceByChannel (.location _returnvalue) (+ (.location _returnvalue) (* (Math|Vector|GetForwardVector (.rotation _returnvalue)) 2e+04)) "TraceTypeQuery1" false 0 "ForDuration")))

(event Input|ActionEvents|InputActionReload
  (params (Key :type Key%20Structure :default "None"))
  ;[0 0.3343 0.9271] Replicated reloading
  (:Pressed
    (if (not (Variables|WeaponSetup|GetReload))
      (Variables|WeaponSetup|SetReload true)
      (CallFunction|MulticastReloadMontage))))

(event Input|ActionEvents|InputActionSwitchweapon
  (params (Key :type Key%20Structure :default "None"))
  ;[0 0.3343 0.9271] Replicated weapon switching
  (:Pressed
    (if (not (Variables|WeaponSetup|GetSwitchingWeapon))
      (Variables|WeaponSetup|SetSwitchingWeapon true)
      (if (== (Variables|WeaponSetup|GetActiveWeapon) (- (Utilities|Array|Length (Variables|WeaponSetup|GetWeaponInventory)) 1))
        (CallFunction|SwitchWeapon)
        (else
          (CallFunction|SwitchWeapon (+ (Variables|WeaponSetup|GetActiveWeapon) 1)))))))

(event Input|AxisEvents|InputAxisMoveForward/Backward
  (params (AxisValue :type Float%20%28single-precision%29))
  ;[0 0.3343 0.9271] Movement
  (Pawn|Input|AddMovementInput (Math|Vector|GetForwardVector (Math|Rotator|MakeRotator 0.0 0.0 (.yaw (Pawn|GetControlRotation :!class /Script/Engine.Pawn)))) AxisValue false))

(event Input|AxisEvents|InputAxisMoveRight/Left
  (params (AxisValue :type Float%20%28single-precision%29))
  (bind _returnvalue (Pawn|GetControlRotation :!class /Script/Engine.Pawn))
  ;[0 0.3343 0.9271] Movement
  (Pawn|Input|AddMovementInput (Math|Vector|GetRightVector (Math|Rotator|MakeRotator (.roll _returnvalue) 0.0 (.yaw _returnvalue))) AxisValue false))

(event Input|AxisEvents|InputAxisTurnRight/LeftMouse
  (params (AxisValue :type Float%20%28single-precision%29))
  ;[0 0.3343 0.9271] Movement
  (Pawn|Input|AddControllerYawInput AxisValue))

(event Input|AxisEvents|InputAxisLookUp/DownMouse
  (params (AxisValue :type Float%20%28single-precision%29))
  ;[0 0.3343 0.9271] Movement
  (Pawn|Input|AddControllerPitchInput AxisValue))

(fn ConstructionScript)

(fn WeaponEffects
  (params (WeaponName :type Name))
  (bind _animationinstance (Variables|AnimationSetup|GetAnimationInstance))
  (bind _returnvalue (Utilities|GetDataTableRow "/Game/Game/Blueprints/Info/WeaponInfoDataTable.WeaponInfoDataTable" WeaponName)
    (:then
      (Class|SkinnedMeshComponent|SetSkeletalMesh (Variables|Default|GetWeaponMesh) (.WeaponMesh (Utilities|Struct|BreakWeaponInfoStruct _returnvalue)) true)
      (Variables|WeaponSetup|SetShooting%20Sound (.ShootingSound (Utilities|Struct|BreakWeaponInfoStruct _returnvalue)))
      (Variables|WeaponSetup|SetMuzzle%20Socket (.MuzzleSocket (Utilities|Struct|BreakWeaponInfoStruct _returnvalue)))
      (Variables|WeaponSetup|SetShell%20Eject%20Socket (.ShellEjectSocket (Utilities|Struct|BreakWeaponInfoStruct _returnvalue)))
      (Variables|Animationsetup|SetWeapon%20Shooting%20Anim (.WeaponShootingAnim (Utilities|Struct|BreakWeaponInfoStruct _returnvalue)))
      (Variables|AnimationSetup|SetWeapon%20Reload%20Anim (.WeaponReloadAnim (Utilities|Struct|BreakWeaponInfoStruct _returnvalue)))
      (Variables|AnimationSetup|SetCharacter%20Shooting%20Anim (.CharacterShootingAnim (Utilities|Struct|BreakWeaponInfoStruct _returnvalue)))
      (Variables|AnimationSetup|SetCharacter%20Reload%20Anim (.CharacterReloadAnim (Utilities|Struct|BreakWeaponInfoStruct _returnvalue)))
      (Variables|WeaponSetup|SetShooting%20Particle (.ShootingParticle (Utilities|Struct|BreakWeaponInfoStruct _returnvalue)))
      (Variables|/Game/Game/Blueprints/AnimationBlueprint.AnimationBlueprint_C|SetCharacterADSIdle _animationinstance (.CharacterADSIdle (Utilities|Struct|BreakWeaponInfoStruct _returnvalue)))
      (Variables|/Game/Game/Blueprints/AnimationBlueprint.AnimationBlueprint_C|SetCharacterHipIdle _animationinstance (.CharacterHipIdle (Utilities|Struct|BreakWeaponInfoStruct _returnvalue)))
      (Variables|/Game/Game/Blueprints/AnimationBlueprint.AnimationBlueprint_C|SetCharacterADSAO _animationinstance (.CharacterADSAO (Utilities|Struct|BreakWeaponInfoStruct _returnvalue)))
      (Variables|/Game/Game/Blueprints/AnimationBlueprint.AnimationBlueprint_C|SetCharacterHipFireAO _animationinstance (.CharacterHipAO (Utilities|Struct|BreakWeaponInfoStruct _returnvalue)))
      (return))))

(fn ServerAddWeaponstoInventory
  (params (InventorySlot :type Integer) (WeaponName :type Name))
  (Utilities|Array|SetArrayElem (Variables|WeaponSetup|GetWeaponInventory) InventorySlot WeaponName true)
  (return))

(fn ServerReplicatedWeaponVariables
  (params (WeaponSlot :type Integer))
  (Variables|WeaponSetup|SetActiveWeapon WeaponSlot)
  (bind _returnvalue (Utilities|GetDataTableRow "/Game/Game/Blueprints/Info/WeaponInfoDataTable.WeaponInfoDataTable" (Utilities|Array|Get(acopy) (Variables|WeaponSetup|GetWeaponInventory) WeaponSlot))
    (:then
      (Variables|WeaponSetup|SetShooting%20Rate (.ShootingRate (Utilities|Struct|BreakWeaponInfoStruct _returnvalue)))
      (Variables|WeaponSetup|SetAuto%20Shooting (.AutoShooting (Utilities|Struct|BreakWeaponInfoStruct _returnvalue)))
      (Variables|WeaponSetup|SetShotgun (.Shotgun (Utilities|Struct|BreakWeaponInfoStruct _returnvalue)))
      (return))))