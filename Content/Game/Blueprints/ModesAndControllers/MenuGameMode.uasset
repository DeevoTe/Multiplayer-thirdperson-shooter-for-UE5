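; Game mode for the menus that tracks players joining the lobby and shares their profiles.
; When a player starts on the Lobby Menu Map, it stores their MenuController and has it create the lobby menu.
; UpdateLobby, gated by its PlayerNames input, rebuilds the profile list from every stored controller and sends it back to each one to refresh displayed player names.
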(event Custom|UpdateLobby
  (params (PlayerNames :type Boolean))
  ;[0 0.3343 0.9271] Update lobby
  (if PlayerNames
    (Utilities|Array|Clear (Variables|Default|GetPlayerProfiles))
    ;;[0.02083 0.02083 0.02083] Displays all connected players
    (for _array_element (Variables|Default|GetAllConnectedPlayers)
      (Utilities|Array|Add (Variables|Default|GetPlayerProfiles) (Variables|/Game/Game/Blueprints/ModesAndControllers/MenuController.MenuController_C|GetPlayerProfileInfo _array_element)))
    (for _array_element_2 (Variables|Default|GetAllConnectedPlayers)
      (if PlayerNames
        (Default|UpdatePlayerNames _array_element_2 (Variables|Default|GetPlayerProfiles))))))

(event EventBeginPlay)

(event EventTick
  (params (DeltaSeconds :type Float%20%28single-precision%29)))

(event EventHandleStartingNewPlayer
  (params (NewPlayer :type Player%20Controller%20Object%20Reference))
  ;[0 0.3343 0.9271] Connect to lobby menu
  (bind _returnvalue (Game|GetCurrentLevelName true))
  (switch string _returnvalue
    (:LobbyMenuMap
      ;;[0.02083 0.02083 0.02083] Checks how many players that is connected
      (bind _asmenu_controller (Utilities|Casting|CastToMenuController NewPlayer))
      (Utilities|Array|Add (Variables|Default|GetAllConnectedPlayers) _asmenu_controller)
      (Default|CreateLobbyMenu _asmenu_controller))))

(fn ConstructionScript)