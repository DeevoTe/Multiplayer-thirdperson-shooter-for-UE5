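; MainGameMode spawns players at indexed player starts and runs the countdown that opens a level.
; HandleStartingNewPlayer collects MainPlayerControllers and reads single-player mode and expected player count from MainGameInstance.
; It spawns one player immediately in single-player, or waits for all expected players before spawning each at the start named by its index.
; StartLevel then triggers each controller's countdown and enables all inputs after a three-second delay.
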(event Custom|StartLevel
  (Utilities|FlowControl|Delay 0.2)
  (for _array_element (Variables|Default|GetAllConnectedPlayerControllers)
    (Default|StartCountdown _array_element)
    (Utilities|FlowControl|Delay 3.0)
    (for _array_element_2 (Variables|Default|GetAllConnectedPlayerControllers)
      (Default|EnableAllInputs _array_element_2))))

(event EventBeginPlay)

(event EventTick
  (params (DeltaSeconds :type Float%20%28single-precision%29)))

(event EventHandleStartingNewPlayer
  (params (NewPlayer :type Player%20Controller%20Object%20Reference))
  (bind _asmain_player_controller (Utilities|Casting|CastToMainPlayerController NewPlayer))
  (Utilities|Array|Add (Variables|Default|GetAllConnectedPlayerControllers) _asmain_player_controller)
  (bind _asmain_game_instance (Utilities|Casting|CastToMainGameInstance (Game|GetGameInstance)))
  (Variables|Default|SetNumberOfExpectedPlayers (Variables|/Game/Game/Blueprints/ModesAndControllers/MainGameInstance.MainGameInstance_C|GetNumber%20Of%20Connected%20Players _asmain_game_instance))
  (if (Variables|/Game/Game/Blueprints/ModesAndControllers/MainGameInstance.MainGameInstance_C|GetSinglePlayer _asmain_game_instance)
    ;[0.01042 0.01042 0.01042] Spawns 1 player if selecting single player game
    (Variables|Default|SetNumberOfExpectedPlayers 1)
    (Class|GameModeBase|RestartPlayeratPlayerStart (Utilities|Array|Get(acopy) (Variables|Default|GetAllConnectedPlayerControllers)) (Class|GameModeBase|FindPlayerStart 0 "0"))
    (CallFunction|StartLevel)
    (elif (== (Variables|Default|GetNumberOfExpectedPlayers) (Utilities|Array|Length (Variables|Default|GetAllConnectedPlayerControllers)))
      (Utilities|FlowControl|Delay 0.1)
      (for (_array_element _array_index) (Variables|Default|GetAllConnectedPlayerControllers)
        (Class|GameModeBase|RestartPlayeratPlayerStart _array_element (Class|GameModeBase|FindPlayerStart _array_element (Utilities|String|ToString(Integer) _array_index))))
      (CallFunction|StartLevel))))

(fn ConstructionScript)