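; Game instance that runs the main and multiplayer menus, the player profile, and single-player or online game startup.
; Opening the main menu loads or creates the saved profile to fill in the player name, and name changes save back to its slot.
; Multiplayer creates a four-connection session with toggleable LAN, opening the lobby as a listen server, or joins a found session.
; Map travel stores the connected player count and runs a ServerTravel console command.
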(event Custom|StartSinglePlayerGame
  ;[0 0.3343 0.9271] Init setup
  (Variables|Default|SetSinglePlayer true)
  (Game|OpenLevel(byName) "Map1"))

(event Custom|ChangePlayerName
  (params (Player%20name :type Text))
  ;[0 0.3343 0.9271] Init setup
  (Variables|Default|SetPlayerProfileInfo (Utilities|Struct|MakePlayerProfileStruct Player%20name))
  (CallFunction|SaveProfile))

(event Custom|CreateMultiplayerSession
  ;[0 0.3343 0.9271] Create / join game
  (Variables|Default|SetSinglePlayer false)
  (|Session (Game|GetPlayerController 0) 4 (Variables|Default|GetLAN)
    (:OnSuccess
      (Game|OpenLevel(byName) "LobbyMenuMap" true "listen"))
    (:OnFailure
      (Development|PrintString "Failed to create session"))))

(event Custom|JoinSession
  (params (Blueprint%20session%20result :type Blueprint%20Session%20Result%20Structure))
  ;[0 0.3343 0.9271] Create / join game
  (Variables|Default|SetSinglePlayer false)
  (|JoinSession (Game|GetPlayerController 0) Blueprint%20session%20result))

(event Custom|TravelToMap
  (params (NumberOfConnectedPlayers :type Integer) (MapName :type String))
  ;[0 0.3343 0.9271] Travel to map
  (Variables|Default|SetNumber%20Of%20Connected%20Players NumberOfConnectedPlayers)
  (Development|ExecuteConsoleCommand (Utilities|String|Append "ServerTravel " MapName) (Game|GetPlayerController 0)))

(fn ShowMainMenu
  (bind _returnvalue (Game|GetPlayerController 0))
  (Utilities|IsValid (Variables|Default|GetMainMenuWidget)
    (:Is%20Not%20Valid
      (bind _returnvalue_2 (UserInterface|CreateWidget "/Game/Game/Blueprints/Widgets/MainMenuWidget.MainMenuWidget_C" _returnvalue))
      (Variables|Default|SetMainMenuWidget _returnvalue_2)
      (UserInterface|Viewport|AddtoViewport (Variables|Default|GetMainMenuWidget) 0)
      (Input|SetInputModeUIOnly _returnvalue 0 "DoNotLock")
      (Variables|/Script/Engine.PlayerController|SetbShowMouseCursor _returnvalue true)
      (CallFunction|CheckSaveProfile)
      (Rendering|Components|TextRender|SetText (Variables|/Game/Game/Blueprints/Widgets/MainMenuWidget.MainMenuWidget_C|GetPlayerNameText (Variables|Default|GetMainMenuWidget)) (Utilities|Struct|BreakPlayerProfileStruct (Variables|Default|GetPlayerProfileInfo)))
      (return))))

(fn LoadProfile
  (bind _returnvalue (SaveGame|LoadGamefromSlot (Variables|Default|GetPlayerProfileSlot)))
  (bind _assave_game_player_profile (Utilities|Casting|CastToSaveGamePlayerProfile _returnvalue))
  (Variables|Default|SetPlayerProfileInfo (Variables|/Game/Game/Blueprints/SaveInfo/SaveGamePlayerProfile.SaveGamePlayerProfile_C|GetPlayerProfile _assave_game_player_profile))
  (return _assave_game_player_profile))

(fn SaveProfile
  (Utilities|IsValid (Variables|Default|GetSaveGamePlayerProfle)
    (:Is%20Valid
      _)
    (:Is%20Not%20Valid
      (bind _returnvalue (SaveGame|CreateSaveGameObject "/Game/Game/Blueprints/SaveInfo/SaveGamePlayerProfile.SaveGamePlayerProfile_C"))
      (Variables|Default|SetSaveGamePlayerProfle _returnvalue)))
  (Variables|/Game/Game/Blueprints/SaveInfo/SaveGamePlayerProfile.SaveGamePlayerProfile_C|SetPlayerProfile (Variables|Default|GetSaveGamePlayerProfle) (Variables|Default|GetPlayerProfileInfo))
  (SaveGame|SaveGametoSlot (Variables|Default|GetSaveGamePlayerProfle) (Variables|Default|GetPlayerProfileSlot))
  (return))

(fn CheckSaveProfile
  (bind _returnvalue (SaveGame|DoesSaveGameExist (Variables|Default|GetPlayerProfileSlot)))
  (if _returnvalue
    (bind _save_game_player_profile (CallFunction|LoadProfile))
    (Variables|Default|SetSaveGamePlayerProfle _save_game_player_profile)
    (else
      (CallFunction|SaveProfile)))
  (return))

(fn ShowMultiplayerMenu
  (Utilities|IsValid (Variables|Default|GetMultiplayerMenuWidget)
    (:Is%20Not%20Valid
      (bind _returnvalue (UserInterface|CreateWidget "/Game/Game/Blueprints/Widgets/MultiplayerWidget.MultiplayerWidget_C"))
      (Variables|Default|SetMultiplayerMenuWidget _returnvalue)
      (UserInterface|Viewport|AddtoViewport (Variables|Default|GetMultiplayerMenuWidget) 0)
      (return))))

(fn ChangeConnectionType
  (if (Variables|Default|GetLAN)
    (Variables|Default|SetLAN false)
    (else
      (Variables|Default|SetLAN true)))
  (return (Variables|Default|GetLAN)))