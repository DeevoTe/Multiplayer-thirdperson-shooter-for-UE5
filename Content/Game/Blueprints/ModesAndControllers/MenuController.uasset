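; Player controller for the menu and multiplayer lobby, handling UI-only mouse input, the lobby and loading-screen widgets, and leaving sessions.
; InitSetup creates a profile save if none exists, loads the profile and passes it through ServerUpdateLobby to MenuGameMode to refresh the lobby.
; Update events push player names and level selection into the lobby widget.
; Destroying the session returns to MainMenuMap.
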(event Custom|UpdatePlayerNames
  (params (PlayerProfiles :type Array%20of%20Player%20Profile%20Struct%20Structures))
  (bind _lobbymenuwidget (Variables|Default|GetLobbyMenuWidget))
  ;[0 0.3343 0.9271] Update player names
  (Utilities|IsValid _lobbymenuwidget
    (:Is%20Valid
      (Default|ClearPlayerNames _lobbymenuwidget)
      (Default|UpdatePlayerName _lobbymenuwidget PlayerProfiles))))

(event Custom|CreateLobbyMenu
  ;[0 0.3343 0.9271] Show lobby menu
  (CallFunction|ShowLobbyMenu))

(event Custom|DestroyClientSession
  ;[0 0.3343 0.9271] End session
  (|DestroySession self
    (:then
      (Game|OpenLevel(byName) "MainMenuMap "))))

(event Custom|InitSetup
  ;[0 0.3343 0.9271] Load profile
  (CallFunction|LoadSavedProfile)
  (CallFunction|ServerUpdateLobby (Variables|Default|GetPlayerProfileInfo)))

(event Custom|ServerUpdateLobby
  (params (PlayerProfile :type Player%20Profile%20Struct%20Structure))
  ;[0 0.3343 0.9271] Update lobby
  (Variables|Default|SetPlayerProfileInfo PlayerProfile)
  (bind _asmenu_game_mode (Utilities|Casting|CastToMenuGameMode (Game|GetGameMode)))
  (Default|UpdateLobby _asmenu_game_mode true true))

(event Custom|CreateLoadScreen
  ;[0 0.3343 0.9271] Show loading screen
  (CallFunction|ShowLoadScreen))

(event Custom|UpdateLevelSelection
  (params (LevelName :type Name))
  (bind _lobbymenuwidget (Variables|Default|GetLobbyMenuWidget))
  ;[0 0.3343 0.9271] Update level selection
  (Utilities|IsValid _lobbymenuwidget
    (:Is%20Valid
      (Default|UpdateLevelSelection _lobbymenuwidget LevelName))))

(event EventBeginPlay
  ;[0 0.3343 0.9271] Begin play
  (if (Pawn|IsLocalController)
    (Variables|Default|SetbShowMouseCursor true)
    (Input|SetInputModeUIOnly self 0 "DoNotLock")))

(fn ConstructionScript)

(fn ShowLobbyMenu
  (Utilities|IsValid (Variables|Default|GetLobbyMenuWidget)
    (:Is%20Valid
      _)
    (:Is%20Not%20Valid
      (bind _returnvalue (UserInterface|CreateWidget "/Game/Game/Blueprints/Widgets/LobbyMenuWidget.LobbyMenuWidget_C" self))
      (Variables|Default|SetLobbyMenuWidget _returnvalue)))
  (UserInterface|Viewport|AddtoViewport (Variables|Default|GetLobbyMenuWidget) 0))

(fn LoadSavedProfile
  (bind _returnvalue (SaveGame|DoesSaveGameExist (LocalVariables|GetLocalSlotName)))
  (if _returnvalue
    _
    (else
      (bind _returnvalue_2 (SaveGame|CreateSaveGameObject "/Game/Game/Blueprints/SaveInfo/SaveGamePlayerProfile.SaveGamePlayerProfile_C"))
      (SaveGame|SaveGametoSlot _returnvalue_2 (LocalVariables|GetLocalSlotName))))
  (bind _returnvalue_3 (SaveGame|LoadGamefromSlot))
  (bind _assave_game_player_profile (Utilities|Casting|CastToSaveGamePlayerProfile _returnvalue_3))
  (Variables|Default|SetPlayerProfileInfo (Variables|/Game/Game/Blueprints/SaveInfo/SaveGamePlayerProfile.SaveGamePlayerProfile_C|GetPlayerProfile _assave_game_player_profile))
  (return))

(fn ShowLoadScreen
  (Viewport|RemoveAllWidgets)
  (Utilities|IsValid (Variables|Default|GetLoadScreenWidget)
    (:Is%20Valid
      _)
    (:Is%20Not%20Valid
      (bind _returnvalue (UserInterface|CreateWidget "/Game/Game/Blueprints/Widgets/LoadingScreenWidget.LoadingScreenWidget_C" self))
      (Variables|Default|SetLoadScreenWidget _returnvalue)))
  (UserInterface|Viewport|AddtoViewport (Variables|Default|GetLoadScreenWidget) 0))